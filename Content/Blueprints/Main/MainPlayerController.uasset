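; Player controller that drives MainPlayerCharacter, translating input into walking, camera look, jumping, sprinting, view switching and weapon pickup.
; On BeginPlay it caches the controlled pawn, sets the initial camera view via FvSetView and binds to the pawn's damage event, which only prints a debug message.
; Speed input swaps max walk speed between run and walk values, and the Action input calls FvTakeWeapon when CurrentWeapon is valid.
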(event Custom|MakeDamage
  (Development|PrintString "I reserved to damage"))

(event EventBeginPlay
  (bind _asmain_player_character (Utilities|Casting|CastToMainPlayerCharacter (Pawn|GetControlledPawn)))
  (Variables|Default|SetMyPawn _asmain_player_character)
  (Development|PrintString "Work")
  (Default|FvSetView (Variables|Default|GetMyPawn) false)
  (EventDispatchers|BindEventtoOnDamage (Variables|Default|GetMyPawn) (delegate Custom|MakeDamage)))

(event EventTick
  (params (DeltaSeconds :type Float%20%28single-precision%29)))

(event Input|ActionEvents|InputActionAction
  (params (Key :type Key%20Structure))
  (:Pressed
    (if (Utilities|IsValid (Variables|/Game/Blueprints/Main/Characters/MainPlayerCharacter.MainPlayerCharacter_C|GetCurrentWeapon (Variables|Default|GetMyPawn)))
      (Default|FvTakeWeapon (Variables|Default|GetMyPawn)))))

(event Input|ActionEvents|InputActionFire
  (params (Key :type Key%20Structure)))

(event Input|ActionEvents|InputActionJump
  (params (Key :type Key%20Structure))
  (:Pressed
    (Character|Jump (Variables|Default|GetMyPawn))))

(event Input|ActionEvents|InputActionSetCameraView
  (params (Key :type Key%20Structure))
  (bind _mypawn (Variables|Default|GetMyPawn))
  (:Pressed
    (Default|FvSetView _mypawn (not (Variables|/Game/Blueprints/Main/Characters/MainPlayerCharacter.MainPlayerCharacter_C|GetCameraView _mypawn)))))

(event Input|ActionEvents|InputActionSpeed
  (params (Key :type Key%20Structure))
  (bind _mypawn (Variables|Default|GetMyPawn))
  (bind _charactermovement (Variables|/Script/Engine.Character|GetCharacterMovement _mypawn))
  (:Pressed
    (Variables|/Script/Engine.CharacterMovementComponent|SetMaxWalkSpeed _charactermovement (Variables|Default|Get@RunSpeed)))
  (:Released
    (Variables|/Script/Engine.CharacterMovementComponent|SetMaxWalkSpeed _charactermovement (Variables|Default|Get@WalkSpeed))))

(event Input|AxisEvents|InputAxisMoveForward
  (params (AxisValue :type Float%20%28single-precision%29))
  ;[1 1 1] Вперед назад
  (Pawn|Input|AddMovementInput (Variables|Default|GetMyPawn) (* (Transformation|GetActorForwardVector (Variables|Default|GetMyPawn)) AxisValue) 1.0 false))

(event Input|AxisEvents|InputAxisMoveRight
  (params (AxisValue :type Float%20%28single-precision%29))
  ;[1 1 1] Лево право
  (Pawn|Input|AddMovementInput (Variables|Default|GetMyPawn) (* (Transformation|GetActorRightVector (Variables|Default|GetMyPawn)) AxisValue) 1.0 false))

(event Input|AxisEvents|InputAxisLookUp
  (params (AxisValue :type Float%20%28single-precision%29))
  ;[1 1 1] Управление камерой
  (Class|PlayerController|AddPitchInput AxisValue))

(event Input|AxisEvents|InputAxisTurnAround
  (params (AxisValue :type Float%20%28single-precision%29))
  ;[1 1 1] Управление камерой
  (Class|PlayerController|AddYawInput AxisValue))

(fn ConstructionScript)